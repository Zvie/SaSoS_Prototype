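; Player projectile actor that moves along a local-space Speed offset each Tick, without sweep, and damages what it overlaps.
; The construction script creates a dynamic material, which BeginPlay tints with ProjectileColor.
; Tick also caches the player Character_Pawn.
; Overlapping any actor other than its owner or itself applies Damage, sets the player's IsProjectile flag and destroys the projectile.
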(event OnComponentBeginOverlap(Projectile)
  (params (OtherActor :type Actor%20Object%20Reference) (OtherComp :type Primitive%20Component%20Object%20Reference) (OtherBodyIndex :type Integer) (bFromSweep :type Boolean) (SweepResult :type Hit%20Result%20Structure%20%28by%20ref%29))
  ;[1 0 0] Apply Damage and Destroy
  (if (and (!= OtherActor (Variables|LEAVEMEALONE|GetProjectileOwner)) (!= OtherActor self))
    (Game|Damage|ApplyDamage OtherActor (Variables|AdjustableVariables|GetDamage) 0 0)
    (Variables|/Game/Blueprints/Character/Character_Pawn.Character_Pawn_C|SetisProjectile (Variables|Default|GetPlayer) true)
    (Actor|DestroyActor)))

(event EventBeginPlay
  ;[0 1 0] Projectile Color
  (Rendering|Material|SetVectorParameterValue (Variables|LEAVEMEALONE|GetProjectileMaterial) "Color2" (Variables|LEAVEMEALONE|GetProjectileColor) :!class /Script/Engine.MaterialInstanceDynamic))

(event EventTick
  (params (DeltaSeconds :type Float%20%28single-precision%29))
  (Utilities|FlowControl|Sequence
    (:then_0
      (Utilities|IsValid (Variables|Default|GetPlayer)
        (:Is%20Not%20Valid
          (bind _ascharacter_pawn (Utilities|Casting|CastToCharacter_Pawn (Game|Player|GetPlayerPawn 0)))
          (Variables|Default|SetPlayer _ascharacter_pawn))))
    (:then_1
      ;[0 0 1] Move Projectile
      (Transformation|AddActorLocalOffset (* (Variables|AdjustableVariables|GetSpeed) DeltaSeconds) false false))))

(fn ConstructionScript
  (bind _returnvalue (Rendering|Material|CreateDynamicMaterialInstance (Variables|Default|GetProjectile) 0 0 :!class /Script/Engine.PrimitiveComponent))
  (Variables|LEAVEMEALONE|SetProjectileMaterial _returnvalue))