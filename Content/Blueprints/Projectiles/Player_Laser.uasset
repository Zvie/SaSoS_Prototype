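; Player laser projectile that fires as a beam attached to its owner and damages other actors it overlaps.
; On BeginPlay it snaps to ProjectileOwner and tints the dynamic material created in the construction script.
; The Movement timeline extends the beam by scaling the Projectile component rather than moving it, then destroys the actor when finished.
; Overlap applies LaserDamage to any actor except the owner; the Player_Projectile check is an unfinished stub.
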(event OnComponentBeginOverlap(Projectile)
  (params (OtherActor :type Actor%20Object%20Reference) (OtherComp :type Primitive%20Component%20Object%20Reference) (OtherBodyIndex :type Integer) (bFromSweep :type Boolean) (SweepResult :type Hit%20Result%20Structure%20%28by%20ref%29))
  ;[1 0 0] Apply Damage
  (if (!= OtherActor (Variables|LEAVEMEALONE|GetProjectileOwner))
    (Game|Damage|ApplyDamage OtherActor (Variables|AdjustableVariables|GetLaserDamage) 0 0)
    (if (stale _bsuccess)
      _)))

(event EventBeginPlay
  ;[0 0 1] Attach to Actor, and Scale
  (Class|Actor|AttachRootComponenttoActor (Variables|LEAVEMEALONE|GetProjectileOwner) "None" "SnapToTarget" true)
  (Rendering|Material|SetVectorParameterValue (Variables|LEAVEMEALONE|GetProjectileMaterial) "Color2" (Variables|LEAVEMEALONE|GetProjectileColor) :!class /Script/Engine.MaterialInstanceDynamic)
  (bind _extend (Timeline|Movement Play)
    (:Update
      (Transformation|SetWorldScale3D (Variables|Default|GetProjectile) _extend))
    (:Finished
      (Actor|DestroyActor))))

(fn ConstructionScript
  (bind _returnvalue (Rendering|Material|CreateDynamicMaterialInstance (Variables|Default|GetProjectile) 0 0 :!class /Script/Engine.PrimitiveComponent))
  (Variables|LEAVEMEALONE|SetProjectileMaterial _returnvalue))