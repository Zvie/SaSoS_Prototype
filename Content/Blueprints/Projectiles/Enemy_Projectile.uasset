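; Enemy projectile actor that flies forward and damages what it hits.
; The construction script creates a dynamic material on the Projectile component, and BeginPlay tints its Color2 parameter with ProjectileColor.
; Tick moves the actor by a local Speed offset scaled by delta time, without sweeping.
; Overlapping any actor other than ProjectileOwner applies Damage and destroys the projectile.
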(event OnComponentBeginOverlap(Projectile)
  (params (OtherActor :type Actor%20Object%20Reference) (OtherComp :type Primitive%20Component%20Object%20Reference) (OtherBodyIndex :type Integer) (bFromSweep :type Boolean) (SweepResult :type Hit%20Result%20Structure%20%28by%20ref%29))
  ;[1 0 0] Apply Damage and Destroy
  (if (!= OtherActor (Variables|LEAVEMEALONE|GetProjectileOwner))
    (Game|Damage|ApplyDamage OtherActor (Variables|AdjustableVariables|GetDamage) 0 0)
    (Actor|DestroyActor)))

(event EventBeginPlay
  ;[0 1 0] Set Projectile Color
  (Rendering|Material|SetVectorParameterValue (Variables|LEAVEMEALONE|GetProjectileMaterial) "Color2" (Variables|LEAVEMEALONE|GetProjectileColor) :!class /Script/Engine.MaterialInstanceDynamic))

(event EventTick
  (params (DeltaSeconds :type Float%20%28single-precision%29))
  ;[0 0 1] Move Projectile
  (Transformation|AddActorLocalOffset (* (Variables|AdjustableVariables|GetSpeed) DeltaSeconds) false false))

(fn ConstructionScript
  (bind _returnvalue (Rendering|Material|CreateDynamicMaterialInstance (Variables|Default|GetProjectile) 0 0 :!class /Script/Engine.PrimitiveComponent))
  (Variables|LEAVEMEALONE|SetProjectileMaterial _returnvalue))