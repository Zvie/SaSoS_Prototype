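; Game controller for a space shooter that runs player lives, enemy spawning, score and boss progression.
; It possesses a spawned player pawn, respawns it on death while lives remain, and otherwise opens game over.
; Tick-driven gates spawn random enemies at offsets, and a collider culls strays.
; Destroy bindings add score toward boss spawns and level changes, though ResetSpawnRate always forces level 1, bypassing the level 2 spawner.
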(event OnComponentBeginOverlap(Collider)
  (params (OverlappedComponent :type Primitive%20Component%20Object%20Reference) (OtherActor :type Actor%20Object%20Reference) (OtherComp :type Primitive%20Component%20Object%20Reference) (OtherBodyIndex :type Integer) (bFromSweep :type Boolean) (SweepResult :type Hit%20Result%20Structure%20%28by%20ref%29))
  ;[1 0 0] Destroy Past Screen Bounds
  (if (Utilities|Array|ContainsItem (Variables|LEAVEMEALONE|GetEnemyArray) OtherActor)
    (Variables|/Game/Blueprints/Character/Character_Pawn.Character_Pawn_C|SetisProjectile (Variables|LEAVEMEALONE|GetPlayer1) false)
    (Actor|DestroyActor OtherActor)))

(event Custom|StopSpawn
  (bind _returnvalue (Transformation|GetActorRotation))
  (bind _returnvalue_2 (Transformation|GetActorRotation))
  (bind _spawnrate_lvl_2 (Variables|AdjustableVariables|GetSpawnRate_Lvl_2))
  (bind _enemyspawnpoint (Variables|Default|GetEnemySpawnPoint))
  (bind _enemyarray (Variables|LEAVEMEALONE|GetEnemyArray))
  (bind _spawnoffset (Variables|LEAVEMEALONE|GetSpawnOffset))
  (bind _actorarray_lvl2 (Variables|AdjustableVariables|GetActorArray_Lvl2))
  (bind _enemyarray_2 (Variables|LEAVEMEALONE|GetEnemyArray))
  (bind _spawnoffset_2 (Variables|LEAVEMEALONE|GetSpawnOffset))
  (bind _actorarray (Variables|AdjustableVariables|GetActorArray))
  (bind _enemyspawnpoint_2 (Variables|Default|GetEnemySpawnPoint))
  (bind _returnvalue_3 (Transformation|GetWorldLocation _enemyspawnpoint))
  (bind _returnvalue_4 (Transformation|GetWorldLocation _enemyspawnpoint_2))
  (bind _returnvalue_5 (* _spawnoffset_2 -1.0))
  (bind _returnvalue_6 (* _spawnoffset -1.0))
  (bind _returnvalue_7 (Math|Random|RandomFloatinRange _returnvalue_6 _spawnoffset))
  (bind _returnvalue_8 (Math|Random|RandomFloatinRange _returnvalue_5 _spawnoffset_2))
  (bind _returnvalue_9 (Math|Vector|MakeVector 0.0 0.0 _returnvalue_7))
  (bind _returnvalue_10 (Math|Vector|MakeVector 0.0 0.0 _returnvalue_8))
  (bind _returnvalue_11 (Math|Vector|UnrotateVector _returnvalue_9 _returnvalue))
  (bind _returnvalue_12 (Math|Vector|UnrotateVector _returnvalue_10 _returnvalue_2))
  (bind _returnvalue_13 (+ _returnvalue_4 _returnvalue_12))
  (bind _returnvalue_14 (+ _returnvalue_3 _returnvalue_11))
  (bind (_x _y _z) (Math|Vector|BreakVector _returnvalue_14))
  (bind (_x_2 _y_2 _z_2) (Math|Vector|BreakVector _returnvalue_13))
  (Utilities|FlowControl|Sequence
    (:then_0
      ;[1 0 0] Enemy Spawning
      (for _array_element _enemyarray_2
        (Utilities|IsValid _array_element
          (:Is%20Valid
            (Actor|DestroyActor _array_element))))
      (Utilities|Array|Clear _enemyarray_2)
      (Utilities|FlowControl|Gate true) ; enters at Close
    )
    (:then_1
      ;[1 0 0] Enemy Spawning
      (for _array_element_2 _enemyarray
        (Utilities|IsValid _array_element_2
          (:Is%20Valid
            (Actor|DestroyActor _array_element_2))))
      (Utilities|Array|Clear _enemyarray)
      (Utilities|FlowControl|Gate true) ; enters at Close
    )))

(event Custom|EnemyKilled
  (params (DestroyedActor :type Actor%20Object%20Reference))
  (Utilities|FlowControl|Sequence
    (:then_0
      (if (Variables|/Game/Blueprints/Character/Character_Pawn.Character_Pawn_C|GetisProjectile (Variables|LEAVEMEALONE|GetPlayer1))
        (if (not (Variables|LEAVEMEALONE|GetisDead))
          (bind _asenemy_3 (Utilities|Casting|CastToEnemy3 (stale EventTick _returnvalue_15))
            (:then
              (Variables|LEAVEMEALONE|SetScore (+ (Variables|LEAVEMEALONE|GetScore) (Variables|/Game/Blueprints/Enemies/Level1_Enemies/Enemy3.Enemy3_C|GetScoreValue _asenemy_3))))
            (:CastFailed
              (bind _asenemy_1 (Utilities|Casting|CastToEnemy1 (stale EventTick _returnvalue_15))
                (:then
                  (Variables|LEAVEMEALONE|SetScore (+ (Variables|LEAVEMEALONE|GetScore) (Variables|/Game/Blueprints/Enemies/Level1_Enemies/Enemy1.Enemy1_C|GetScoreValue _asenemy_1))))
                (:CastFailed
                  (bind _asenemy_2 (Utilities|Casting|CastToEnemy2 (stale EventTick _returnvalue_15))
                    (:then
                      (Variables|LEAVEMEALONE|SetScore (+ (Variables|LEAVEMEALONE|GetScore) (Variables|/Game/Blueprints/Enemies/Level1_Enemies/Enemy2.Enemy2_C|GetScoreValue _asenemy_2))))
                    (:CastFailed
                      (bind _asturret_enemy (Utilities|Casting|CastToTurret_Enemy (stale EventTick _returnvalue_15))
                        (:then
                          (Variables|LEAVEMEALONE|SetScore (+ (Variables|LEAVEMEALONE|GetScore) (Variables|/Game/Blueprints/Enemies/Level1_Enemies/Turret_Enemy.Turret_Enemy_C|GetScoreValue _asturret_enemy))))
                        (:CastFailed
                          _))))))))
          (if (>= (Variables|LEAVEMEALONE|GetScore) (Variables|AdjustableVariables|GetBossScore))
            ;[1 1 1] Boss Notification Widget
            (Development|PrintString "INCOMING BOSS!!!!")
            (Utilities|Array|Clear (Variables|AdjustableVariables|GetActorArray))
            ;[1 0 1] Boss
            (Utilities|FlowControl|Delay 5.0)
            (Utilities|FlowControl|DoOnce false
              (:Completed
                (bind _returnvalue (Game|SpawnActorfromClass "/Game/Blueprints/Enemies/Level1_Enemies/Boss_Enemy.Boss_Enemy_C" (Transformation|GetWorldTransform (Variables|Default|GetEnemySpawnPoint)) "Undefined" 0 0))
                (bind _output_get (Variables|LEAVEMEALONE|SetBossEnemy _returnvalue))
                (Game|BindEventtoOnDestroyed _output_get (delegate Custom|GameWon))))))))
    (:then_1
      (if (Variables|/Game/Blueprints/Character/Character_Pawn.Character_Pawn_C|GetisProjectile (Variables|LEAVEMEALONE|GetPlayer1))
        (if (not (Variables|LEAVEMEALONE|GetisDead))
          (bind _asenemy_1_lvl_2 (Utilities|Casting|CastToEnemy1_lvl2 (stale EventTick _returnvalue_16))
            (:then
              (Variables|LEAVEMEALONE|SetScore (+ (Variables|LEAVEMEALONE|GetScore) (Variables|/Game/Blueprints/Enemies/Levle2_Enemies/Enemy1_lvl2.Enemy1_lvl2_C|GetScoreValue _asenemy_1_lvl_2)))
              (if (>= (Variables|LEAVEMEALONE|GetScore) (Variables|AdjustableVariables|GetLvl2_BossScore)) :!label _label
                ;[1 1 1] Boss Notification Widget
                (Development|PrintString "INCOMING BOSS!!!!")
                (Utilities|Array|Clear (Variables|AdjustableVariables|GetActorArray))
                ;[1 0 1] Boss
                (Utilities|FlowControl|Delay 5.0)
                (Utilities|FlowControl|DoOnce false
                  (:Completed
                    (Game|SpawnActorfromClass "/Game/Blueprints/Enemies/Levle2_Enemies/Boss_Enemy_lvl2.Boss_Enemy_lvl2_C" (Transformation|GetWorldTransform (Variables|Default|GetEnemySpawnPoint)) "Undefined" 0 0)
                    (bind _output_get_2 (Variables|LEAVEMEALONE|SetBossEnemy 0))
                    (Game|BindEventtoOnDestroyed _output_get_2 (delegate Custom|CustomEvent))))))
            (:CastFailed
              (bind _asenemy_2_lvl_2 (Utilities|Casting|CastToEnemy2_lvl2 (stale EventTick _returnvalue_16))
                (:then
                  (Variables|LEAVEMEALONE|SetScore (+ (Variables|LEAVEMEALONE|GetScore) (Variables|/Game/Blueprints/Enemies/Levle2_Enemies/Enemy2_lvl2.Enemy2_lvl2_C|GetScoreValue _asenemy_2_lvl_2)))
                  (goto _label))
                (:CastFailed
                  (bind _asenemy_3_lvl_2 (Utilities|Casting|CastToEnemy3_lvl2 (stale EventTick _returnvalue_16))
                    (:then
                      (Variables|LEAVEMEALONE|SetScore (+ (Variables|LEAVEMEALONE|GetScore) (Variables|/Game/Blueprints/Enemies/Levle2_Enemies/Enemy3_lvl2.Enemy3_lvl2_C|GetScoreValue _asenemy_3_lvl_2)))
                      (goto _label))
                    (:CastFailed
                      (bind _asturret_enemy_lvl_2 (Utilities|Casting|CastToTurret_Enemy_lvl2 (stale EventTick _returnvalue_16))
                        (:then
                          (Variables|LEAVEMEALONE|SetScore (+ (Variables|LEAVEMEALONE|GetScore) (Variables|/Game/Blueprints/Enemies/Levle2_Enemies/Turret_Enemy_lvl2.Turret_Enemy_lvl2_C|GetScoreValue _asturret_enemy_lvl_2))))
                        (:CastFailed
                          (goto _label))))))))))))))

(event Custom|CustomEvent
  (params (DestroyedActor :type Actor%20Object%20Reference))
  ;[1 0 0.1885] Open Game Won Level
  (Variables|LEAVEMEALONE|SetisNextLevel true)
  (Utilities|FlowControl|Delay 5.0)
  (Game|OpenLevel(byName) (Variables|AdjustableVariables|GetGameWonLevelName)))

(event Custom|PlayerDeath
  (params (DestroyedActor :type Actor%20Object%20Reference))
  ;[1 0 0] Death'
  (Variables|LEAVEMEALONE|SetisDead true)
  (Variables|LEAVEMEALONE|SetLives (- (Variables|LEAVEMEALONE|GetLives) 1))
  (CallFunction|StopSpawn)
  (Game|Player|SetViewTargetwithBlend (Game|GetPlayerController 0) self 0.0 "VTBlend_Linear" 0.0 false)
  (Utilities|FlowControl|Gate true
    (:Exit
      (if (> (Variables|LEAVEMEALONE|GetLives) 0)
        (CallFunction|BeginPlay)
        (else
          (Game|OpenLevel(byName) (Variables|AdjustableVariables|GetGameOverLevelName)))))))

(event Custom|GameWon
  (params (DestroyedActor :type Actor%20Object%20Reference))
  ;[1 0 0.1885] Open Game Won Level
  (Variables|LEAVEMEALONE|SetisNextLevel true)
  (Variables|LEAVEMEALONE|SetisLevel2 true)
  (Variables|LEAVEMEALONE|SetisLevel1 false)
  (Utilities|FlowControl|Delay 5.0)
  (Game|OpenLevel(byName) (Variables|LEAVEMEALONE|Getgmwonlvl2)))

(event Custom|Reset%20Spawn%20Rate
  (bind _returnvalue (Transformation|GetActorRotation))
  (bind _returnvalue_2 (Transformation|GetActorRotation))
  (bind _spawnrate_lvl_2 (Variables|AdjustableVariables|GetSpawnRate_Lvl_2))
  (bind _enemyspawnpoint (Variables|Default|GetEnemySpawnPoint))
  (bind _spawnoffset (Variables|LEAVEMEALONE|GetSpawnOffset))
  (bind _actorarray_lvl2 (Variables|AdjustableVariables|GetActorArray_Lvl2))
  (bind _spawnoffset_2 (Variables|LEAVEMEALONE|GetSpawnOffset))
  (bind _actorarray (Variables|AdjustableVariables|GetActorArray))
  (bind _enemyspawnpoint_2 (Variables|Default|GetEnemySpawnPoint))
  (bind _returnvalue_3 (Transformation|GetWorldLocation _enemyspawnpoint))
  (bind _returnvalue_4 (Transformation|GetWorldLocation _enemyspawnpoint_2))
  (bind _returnvalue_5 (* _spawnoffset_2 -1.0))
  (bind _returnvalue_6 (* _spawnoffset -1.0))
  (bind _returnvalue_7 (Math|Random|RandomFloatinRange _returnvalue_6 _spawnoffset))
  (bind _returnvalue_8 (Math|Random|RandomFloatinRange _returnvalue_5 _spawnoffset_2))
  (bind _returnvalue_9 (Math|Vector|MakeVector 0.0 0.0 _returnvalue_7))
  (bind _returnvalue_10 (Math|Vector|MakeVector 0.0 0.0 _returnvalue_8))
  (bind _returnvalue_11 (Math|Vector|UnrotateVector _returnvalue_9 _returnvalue))
  (bind _returnvalue_12 (Math|Vector|UnrotateVector _returnvalue_10 _returnvalue_2))
  (bind _returnvalue_13 (+ _returnvalue_4 _returnvalue_12))
  (bind _returnvalue_14 (+ _returnvalue_3 _returnvalue_11))
  (bind (_x _y _z) (Math|Vector|BreakVector _returnvalue_14))
  (bind (_x_2 _y_2 _z_2) (Math|Vector|BreakVector _returnvalue_13))
  (bind _output_get (Variables|LEAVEMEALONE|SetisLevel1 true))
  (if _output_get
    ;[1 0 0] Enemy Spawning
    (Utilities|FlowControl|Gate true) ; enters at Open
    (else
      ;[1 0 0] Enemy Spawning
      (if (Variables|LEAVEMEALONE|GetisLevel2)
        (Utilities|FlowControl|Gate true) ; enters at Open
      ))))

(event Custom|BeginPlay
  (bind _returnvalue (Game|GetPlayerController 0))
  ;[0 1 0] Custom Event Begin Play
  (Variables|LEAVEMEALONE|SetisDead true)
  (Utilities|FlowControl|Sequence
    (:then_0
      ;[0 0 1] Begin Spawn
      (Variables|AdjustableVariables|SetSpawnRate 1.0)
      (CallFunction|ResetSpawnRate)
      (bind _returnvalue_2 (Game|SpawnActorfromClass "/Game/Blueprints/Character/Character_Pawn.Character_Pawn_C" (Transformation|GetWorldTransform (Variables|Default|GetPlayerSpawnPoint)) "Undefined" 0 0))
      (Variables|LEAVEMEALONE|SetisDead false)
      (bind _output_get (Variables|LEAVEMEALONE|SetPlayer _returnvalue_2))
      (Pawn|Possess _returnvalue _output_get)
      (Game|BindEventtoOnDestroyed (Variables|LEAVEMEALONE|GetPlayer) (delegate Custom|PlayerDeath))
      (Game|Player|SetViewTargetwithBlend _returnvalue self 0.0 "VTBlend_Linear" 0.0 false)
      (bind _ascharacter_pawn (Utilities|Casting|CastToCharacter_Pawn (Game|Player|GetPlayerPawn 0)))
      (Variables|LEAVEMEALONE|SetPlayer1 _ascharacter_pawn))
    (:then_1
      ;[1 0 0] Death'
      (Utilities|FlowControl|Gate true) ; enters at Open
    )))

(event Custom|QuitGame
  ;[1 0 0] Death'
  (Utilities|FlowControl|Sequence
    (:then_0
      (Utilities|FlowControl|Gate true) ; enters at Close
    )
    (:then_1
      (Actor|DestroyActor (Variables|LEAVEMEALONE|GetPlayer)))))

(event EventBeginPlay
  ;[0 1 0] Begin Play
  (bind _returnvalue (UserInterface|CreateWidget "/Game/Blueprints/Widgets/Main_HUD.Main_HUD_C" 0 self))
  (UserInterface|Viewport|AddtoViewport _returnvalue 0)
  (CallFunction|BeginPlay))

(event EventTick
  (params (DeltaSeconds :type Float%20%28single-precision%29))
  (bind _returnvalue (Transformation|GetActorRotation))
  (bind _returnvalue_2 (Transformation|GetActorRotation))
  (bind _spawnrate_lvl_2 (Variables|AdjustableVariables|GetSpawnRate_Lvl_2))
  (bind _enemyspawnpoint (Variables|Default|GetEnemySpawnPoint))
  (bind _spawnoffset (Variables|LEAVEMEALONE|GetSpawnOffset))
  (bind _actorarray_lvl2 (Variables|AdjustableVariables|GetActorArray_Lvl2))
  (bind _spawnoffset_2 (Variables|LEAVEMEALONE|GetSpawnOffset))
  (bind _actorarray (Variables|AdjustableVariables|GetActorArray))
  (bind _enemyspawnpoint_2 (Variables|Default|GetEnemySpawnPoint))
  (bind _player1 (Variables|LEAVEMEALONE|GetPlayer1))
  (bind _returnvalue_3 (Transformation|GetWorldLocation _enemyspawnpoint))
  (bind _returnvalue_4 (Transformation|GetWorldLocation _enemyspawnpoint_2))
  (bind _returnvalue_5 (* _spawnoffset_2 -1.0))
  (bind _returnvalue_6 (* _spawnoffset -1.0))
  (bind _returnvalue_7 (Math|Random|RandomFloatinRange _returnvalue_6 _spawnoffset))
  (bind _returnvalue_8 (Math|Random|RandomFloatinRange _returnvalue_5 _spawnoffset_2))
  (bind _returnvalue_9 (Math|Vector|MakeVector 0.0 0.0 _returnvalue_7))
  (bind _returnvalue_10 (Math|Vector|MakeVector 0.0 0.0 _returnvalue_8))
  (bind _returnvalue_11 (Math|Vector|UnrotateVector _returnvalue_9 _returnvalue))
  (bind _returnvalue_12 (Math|Vector|UnrotateVector _returnvalue_10 _returnvalue_2))
  (bind _returnvalue_13 (+ _returnvalue_4 _returnvalue_12))
  (bind _returnvalue_14 (+ _returnvalue_3 _returnvalue_11))
  (bind (_x _y _z) (Math|Vector|BreakVector _returnvalue_14))
  (bind (_x_2 _y_2 _z_2) (Math|Vector|BreakVector _returnvalue_13))
  ;[1 1 1] Move Player After Win
  (Utilities|FlowControl|Sequence
    (:then_0
      ;[1 0 0] Enemy Spawning
      (Utilities|FlowControl|Gate true
        (:Exit
          (Utilities|FlowControl|Delay (Math|Random|RandomFloatinRange (Variables|AdjustableVariables|GetSpawnRate) (+ (Variables|AdjustableVariables|GetSpawnRate) 0.1)))
          (bind _returnvalue_15 (Game|SpawnActorfromClass (Utilities|Array|Get(acopy) _actorarray (Math|Random|RandomInteger (Utilities|Array|Length _actorarray))) (Math|Transform|MakeTransform (Math|Vector|MakeVector _x_2 _y_2 _z_2) (Transformation|GetWorldRotation _enemyspawnpoint_2)) "AlwaysSpawn" 0 0))
          (Utilities|Array|Add (Variables|LEAVEMEALONE|GetEnemyArray) _returnvalue_15)
          (Utilities|IsValid _returnvalue_15
            (:Is%20Valid
              (Game|BindEventtoOnDestroyed _returnvalue_15 (delegate Custom|EnemyKilled))
              (Variables|AdjustableVariables|SetSpawnRate (Math|Float|Clamp(Float) (+ (Variables|AdjustableVariables|GetSpawnRate) 0.3))))))))
    (:then_1
      ;[1 0 0] Enemy Spawning
      (Utilities|FlowControl|Gate true
        (:Exit
          (Utilities|FlowControl|Delay (Math|Random|RandomFloatinRange _spawnrate_lvl_2 (+ _spawnrate_lvl_2 0.1)))
          (bind _returnvalue_16 (Game|SpawnActorfromClass (Utilities|Array|Get(acopy) _actorarray_lvl2 (Math|Random|RandomInteger (Utilities|Array|Length _actorarray_lvl2))) (Math|Transform|MakeTransform (Math|Vector|MakeVector _x _y _z) (Transformation|GetWorldRotation _enemyspawnpoint)) "AlwaysSpawn" 0 0))
          (Utilities|Array|Add (Variables|LEAVEMEALONE|GetEnemyArray) _returnvalue_16)
          (Utilities|IsValid _returnvalue_16
            (:Is%20Valid
              (Game|BindEventtoOnDestroyed _returnvalue_16 (delegate Custom|EnemyKilled))
              (Variables|AdjustableVariables|SetSpawnRate (Math|Float|Clamp(Float) (+ (Variables|AdjustableVariables|GetSpawnRate) 0.3))))))))
    (:then_2
      (if (Variables|LEAVEMEALONE|GetGameWon!)
        (Utilities|FlowControl|Delay 2.0)
        (bind _returndirection (Default|PlayerMovement _player1 1.0 -5e+01))
        (Variables|/Game/Blueprints/Character/Character_Pawn.Character_Pawn_C|SetHorizontalSpeed _player1 _returndirection)))))

(fn ConstructionScript
  (Transformation|SetRelativeLocation (Variables|Default|GetCollider) (Variables|AdjustableVariables|GetTriggerLocation) false false)
  (Transformation|SetRelativeLocation (Variables|Default|GetPlayerSpawnPoint) (Variables|AdjustableVariables|GetPlayerSpawn) false false)
  (Transformation|SetRelativeLocation (Variables|Default|GetEnemySpawnPoint) (Variables|AdjustableVariables|GetEnemySpawn) false false))