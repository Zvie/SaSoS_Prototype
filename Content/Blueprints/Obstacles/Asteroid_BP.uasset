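; Asteroid obstacle Blueprint that drifts, damages pawns it hits and can be destroyed.
; Tick plays a timeline whose track supplies vertical velocity alongside a constant X speed, moving the actor without sweep.
; Hit applies damage to pawns, while incoming damage lowers clamped health and at zero swaps the Paper2D flipbook before a delayed destroy.
; Random sprite scaling exists in the construction script but is disconnected.
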(event EventTick
  (params (DeltaSeconds :type Float%20%28single-precision%29))
  ;[0 0 1] Asteroid Movement
  (bind _hozmove (Timeline|HozMovement Play)
    (:Update
      (Transformation|SetActorLocation (+ (Transformation|GetActorLocation) (* (Math|Vector|MakeVector (Variables|Default|GetMoveSpeed) 0.0 _hozmove) DeltaSeconds)) false false))))

(event Collision|EventHit
  (params (MyComp :type Primitive%20Component%20Object%20Reference) (Other :type Actor%20Object%20Reference) (OtherComp :type Primitive%20Component%20Object%20Reference) (bSelfMoved :type Boolean) (HitLocation :type Vector :default "0, 0, 0") (HitNormal :type Vector :default "0, 0, 0") (NormalImpulse :type Vector :default "0, 0, 0") (Hit :type Hit%20Result%20Structure%20%28by%20ref%29))
  ;[1 0 0] Deal Damage
  (bind _aspawn (Utilities|Casting|CastToPawn Other))
  (Game|Damage|ApplyDamage _aspawn (Variables|Default|GetDamage) 0 0))

(event Game|Damage|EventAnyDamage
  (params (Damage :type Float%20%28single-precision%29) (DamageType :type Damage%20Type%20Object%20Reference) (InstigatedBy :type Controller%20Object%20Reference) (DamageCauser :type Actor%20Object%20Reference))
  ;[1 0 0] Take Damage & Death
  (Variables|Default|SetHealth (Math|Float|Clamp(Float) (- (Variables|Default|GetHealth) Damage)))
  (if (<= (Variables|Default|GetHealth) 0.0)
    (Sprite|SetFlipbook (Variables|Default|GetAsteroidFlipbook) "/Game/Trevino_Content/Trevino_Flipbbooks/Level/Trevino_Asteriod_FB.Trevino_Asteriod_FB")
    (Utilities|FlowControl|Delay 0.2)
    (Actor|DestroyActor)))

(fn ConstructionScript)