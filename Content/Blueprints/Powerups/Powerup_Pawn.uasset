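; Temporary ship powerup pawn that snaps onto the player's Character_Pawn as an auxiliary gun.
; On BeginPlay it attaches to player 0's pawn, then destroys itself after ShipPowerupDelay.
; Tick uses a Delay as a fire timer, spawning tinted Player_Projectiles from four fire points with itself as owner.
; An interpolated PlayerMovement helper is defined but not called in this Blueprint.
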(event EventBeginPlay
  ;[0 1 0] Begin Play
  (bind _ascharacter_pawn (Utilities|Casting|CastToCharacter_Pawn (Game|Player|GetPlayerPawn 0)))
  (Class|Actor|AttachRootComponenttoActor _ascharacter_pawn "None" "SnapToTarget" true)
  (Utilities|FlowControl|Delay (Variables|AdjustableVariables|GetShipPowerupDelay))
  (Actor|DestroyActor))

(event EventTick
  (params (DeltaSeconds :type Float%20%28single-precision%29))
  ;[1 0 0] Fire Timer
  (Utilities|FlowControl|Delay (Variables|AdjustableVariables|GetFireDelay))
  (CallFunction|PrimaryFire (Variables|Default|GetFire1))
  (CallFunction|PrimaryFire (Variables|Default|GetFire3))
  (CallFunction|PrimaryFire (Variables|Default|GetFire2))
  (CallFunction|PrimaryFire (Variables|Default|GetFire4)))

(fn ConstructionScript)

(fn PlayerMovement
  (params (Direction :type Float%20%28single-precision%29) (Speed :type Float%20%28single-precision%29))
  ;[0 0 1] Player Movement Function
  (bind _output_get (Variables|LEAVEMEALONE|SetCurrentSpeed (Math|Interpolation|FInterpTo Speed (* (* Direction (Variables|LEAVEMEALONE|GetMovementSpeed)) (Variables|LEAVEMEALONE|GetDeltaSeconds)) (Variables|LEAVEMEALONE|GetDeltaSeconds) 4.0)))
  (return _output_get))

(fn PrimaryFire
  (params (Location :type Scene%20Component%20Object%20Reference))
  ;[1 0 0] Primary Fire Function
  (Game|SpawnActorfromClass "/Game/Blueprints/Projectiles/Player_Projectile.Player_Projectile_C" (Transformation|GetWorldTransform Location) "Undefined" 0 (Math|Color|MakeColor 0.6 0.3 0.6 1.0) (Math|Vector|MakeVector 7e+02 0.0 0.0) self))