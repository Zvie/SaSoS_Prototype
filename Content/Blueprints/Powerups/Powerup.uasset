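; Powerup pickup actor that randomly becomes a health, spinning laser or ship powerup on BeginPlay and shows the matching sprite.
; It drifts along X at MoveSpeed, with a timeline supplying Z motion.
; On hit by Character_Pawn it refills health, sets PowerupVar for the laser, or sets PowerupVar and restores a life below the cap, then destroys itself.
; Damage lowers its Health, but zero health triggers nothing.
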(event EventTick
  (params (DeltaSeconds :type Float%20%28single-precision%29))
  ;[0 0 1] PowerUp Movement
  (bind _hozmove (Timeline|HozMovement Play)
    (:Update
      (Transformation|SetActorLocation (+ (Transformation|GetActorLocation) (* (Math|Vector|MakeVector (Variables|AdjustableVariables|GetMoveSpeed) 0.0 _hozmove) DeltaSeconds)) false false))))

(event Collision|EventHit
  (params (MyComp :type Primitive%20Component%20Object%20Reference) (Other :type Actor%20Object%20Reference) (OtherComp :type Primitive%20Component%20Object%20Reference) (bSelfMoved :type Boolean) (HitLocation :type Vector :default "0, 0, 0") (HitNormal :type Vector :default "0, 0, 0") (NormalImpulse :type Vector :default "0, 0, 0") (Hit :type Hit%20Result%20Structure%20%28by%20ref%29))
  ;[0 1 0] Give Bonus
  ;;[1 1 1] Event Hit
  (bind _ascharacter_pawn (Utilities|Casting|CastToCharacter_Pawn Other))
  (Variables|LEAVEMEALONE|SetPlayer _ascharacter_pawn)
  (if (== Other (Variables|LEAVEMEALONE|GetPlayer))
    ;;[1 1 1] Restore Health Powerup
    (if (== (Variables|LEAVEMEALONE|GetpowerInt) 0)
      (Variables|/Game/Blueprints/Character/Character_Pawn.Character_Pawn_C|SetPlayerHealth (Variables|LEAVEMEALONE|GetPlayer) (Variables|/Game/Blueprints/Character/Character_Pawn.Character_Pawn_C|GetMaxHealth (Variables|LEAVEMEALONE|GetPlayer)))
      (Development|PrintString "Health Added" true true "(R=0.000000,G=1.000000,B=0.000000,A=1.000000)")
      (Actor|DestroyActor)
      (else
        ;;[1 1 1] Spinning Laser Powerup
        (if (== (Variables|LEAVEMEALONE|GetpowerInt) 1)
          (Variables|/Game/Blueprints/Character/Character_Pawn.Character_Pawn_C|SetPowerupVar (Variables|LEAVEMEALONE|GetPlayer) 1)
          (Actor|DestroyActor)
          (else
            ;;[1 1 1] Ship Powerup
            (if (== (Variables|LEAVEMEALONE|GetpowerInt) 2)
              (Variables|/Game/Blueprints/Character/Character_Pawn.Character_Pawn_C|SetPowerupVar (Variables|LEAVEMEALONE|GetPlayer) 2)
              (if (< (Variables|/Game/Blueprints/GameFiles/SpaceTemplate_GameController.SpaceTemplate_GameController_C|GetLives (Variables|Default|GetGameController)) 3)
                (Development|PrintString "Live Restored" true true "(R=0.000000,G=1.000000,B=0.000000,A=1.000000)")
                (Variables|/Game/Blueprints/GameFiles/SpaceTemplate_GameController.SpaceTemplate_GameController_C|SetLives (Variables|Default|GetGameController) (+ (Variables|/Game/Blueprints/GameFiles/SpaceTemplate_GameController.SpaceTemplate_GameController_C|GetLives (Variables|Default|GetGameController)) 1))
                (Actor|DestroyActor)
                (else
                  (Development|PrintString "Lives are Full already" true true "(R=0.000000,G=1.000000,B=0.000000,A=1.000000)")
                  (Actor|DestroyActor))))))))))

(event Game|Damage|EventAnyDamage
  (params (Damage :type Float%20%28single-precision%29) (DamageType :type Damage%20Type%20Object%20Reference) (InstigatedBy :type Controller%20Object%20Reference) (DamageCauser :type Actor%20Object%20Reference))
  ;[1 0 0] Collision Death
  (Variables|LEAVEMEALONE|SetHealth (Math|Float|Clamp(Float) (- (Variables|LEAVEMEALONE|GetHealth) Damage)))
  (if (<= (Variables|LEAVEMEALONE|GetHealth) 0.0)
    _))

(event EventBeginPlay
  ;[1 1 1] Pick Powerup
  (Variables|LEAVEMEALONE|SetpowerInt (Math|Random|RandomInteger (Utilities|Array|Length (Variables|LEAVEMEALONE|GetPowerUpArray))))
  ;[1 1 1] Set Powerup Sprite
  (if (== (Variables|LEAVEMEALONE|GetpowerInt) 0)
    (Rendering|Components|Sprite|SetSprite (Variables|Default|GetPowerupSprite) (Variables|AdjustableVariables|GetHealthPowerup))
    (elif (== (Variables|LEAVEMEALONE|GetpowerInt) 1)
      (Rendering|Components|Sprite|SetSprite (Variables|Default|GetPowerupSprite) (Variables|AdjustableVariables|GetLaserPowerup))
      (elif (== (Variables|LEAVEMEALONE|GetpowerInt) 2)
        (Rendering|Components|Sprite|SetSprite (Variables|Default|GetPowerupSprite) (Variables|AdjustableVariables|GetShipPowerup))))))

(fn ConstructionScript)