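; Player ship pawn for a shooter, with spin-in spawn animation, planar movement, weapons, powerups and health.
; Tick eases horizontal and vertical speeds toward input, then applies a swept move rotated by the spawn yaw.
; Primary fire uses a looping timer for twin projectiles; the laser recharges via timeline.
; Powerups spawn a spinning laser or helper pawn; damage is ignored until shortly after spawning, and death triggers an explosion.
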(event Custom|FireDown
  ;[1 0 0] Fire Timer
  (bind _returnvalue (Utilities|Time|SetTimerbyFunctionName 0 "FireReset" (Variables|AdjustableVariables|GetFireRate) true))
  (Variables|LEAVEMEALONE|SetTimeHandler _returnvalue)
  (CallFunction|PrimaryFire (Variables|Default|GetTopProjectileSpawn))
  (CallFunction|PrimaryFire (Variables|Default|GetBottomProjectileSpawn)))

(event Custom|FireUp
  ;[1 0 0] Fire Timer
  (Utilities|Time|ClearandInvalidateTimerbyHandle (Variables|LEAVEMEALONE|GetTimeHandler)))

(event Custom|Fire2
  ;[1 0 0] FireLaser
  (if (Variables|LEAVEMEALONE|GetLaserReady)
    (Variables|LEAVEMEALONE|SetLaserReady false)
    (Game|SpawnActorfromClass "/Game/Blueprints/Projectiles/Player_Laser.Player_Laser_C" (Transformation|GetWorldTransform (Variables|Default|GetLaserSpawn)) "Undefined" 0 (Math|Color|MakeColor 0.2 0.2 1.0 1.0) self)
    (Timeline|Timeline_0 PlayFromStart
      (:Finished
        (Utilities|IsValid self
          (:Is%20Valid
            (Variables|LEAVEMEALONE|SetLaserReady true))
          (:Is%20Not%20Valid
            (CallFunction|Respawn)))))))

(event Custom|Respawn
  ;[0 0 1] Spawn Anim
  (Utilities|FlowControl|Sequence
    (:then_0
      (Variables|Default|SetcanBeDamaged false)
      (Variables|LEAVEMEALONE|SetYaw (.Yaw (Math|Rotator|BreakRotator (Transformation|GetActorRotation (Game|GetInstigator)))))
      (Variables|LEAVEMEALONE|SetSpawnLocation (Transformation|GetActorLocation))
      (bind _lerp (Timeline|Spawn%20Anim Play)
        (:Update
          (Transformation|SetActorLocation (Math|Vector|Lerp(Vector) (Variables|LEAVEMEALONE|GetSpawnLocation) (+ (Variables|LEAVEMEALONE|GetSpawnLocation) "60.000000, 0,0.000000") _lerp) true false)
          (Transformation|SetActorRotation (Math|Rotator|Lerp(Rotator) "0, 0, 0" (Math|Rotator|MakeRotator 0.0 0.0 (+ 7.2e+02 (Variables|LEAVEMEALONE|GetYaw))) _lerp)))
        (:Finished
          (Variables|LEAVEMEALONE|SetcanMove true)
          (Utilities|FlowControl|Delay 0.2)
          (Variables|Default|SetcanBeDamaged true))))))

(event Custom|UsePowerup
  ;[0 1 0] Powerup Event
  ;[0 1 0] Laser Powerup
  (if (== (Variables|LEAVEMEALONE|GetPowerupVar) 1)
    (bind _returnvalue (Game|SpawnActorfromClass "/Game/Blueprints/Projectiles/Player_Laser.Player_Laser_C" (Transformation|GetWorldTransform (Variables|Default|GetLaserSpawn)) "Undefined" 0 (Math|Color|MakeColor 0.0 0.0 0.0) self))
    (Variables|/Script/Engine.RotatingMovementComponent|SetRotationRate (Variables|/Game/Blueprints/Projectiles/Player_Laser.Player_Laser_C|GetRotatingMovement _returnvalue) "0, 0,360.000000")
    (Variables|LEAVEMEALONE|SetPowerupVar 0)
    (else
      ;[0 1 0] Ship Powerup
      (if (== (Variables|LEAVEMEALONE|GetPowerupVar) 2)
        (bind _returnvalue_2 (Game|SpawnActorfromClass "/Game/Blueprints/Powerups/Powerup_Pawn.Powerup_Pawn_C" (Math|Transform|MakeTransform (.Location (Math|Transform|BreakTransform (Transformation|GetWorldTransform (Variables|Default|GetPowerupShipSpawn)))) "0, 0, 0" "1.000000,1.000000,1.000000") "Undefined" 0 0))
        (Variables|LEAVEMEALONE|SetPowerupVar 0)))))

(event Custom|FireReset
  ;[1 0 0] Fire Timer
  (CallFunction|PrimaryFire (Variables|Default|GetTopProjectileSpawn))
  (CallFunction|PrimaryFire (Variables|Default|GetBottomProjectileSpawn)))

(event EventBeginPlay
  ;[0 0 1] Spawn Anim
  (Utilities|FlowControl|Sequence
    (:then_0
      (Variables|Default|SetcanBeDamaged false)
      (Variables|LEAVEMEALONE|SetYaw (.Yaw (Math|Rotator|BreakRotator (Transformation|GetActorRotation (Game|GetInstigator)))))
      (Variables|LEAVEMEALONE|SetSpawnLocation (Transformation|GetActorLocation))
      (bind _lerp (Timeline|Spawn%20Anim Play)
        (:Update
          (Transformation|SetActorLocation (Math|Vector|Lerp(Vector) (Variables|LEAVEMEALONE|GetSpawnLocation) (+ (Variables|LEAVEMEALONE|GetSpawnLocation) "60.000000, 0,0.000000") _lerp) true false)
          (Transformation|SetActorRotation (Math|Rotator|Lerp(Rotator) "0, 0, 0" (Math|Rotator|MakeRotator 0.0 0.0 (+ 7.2e+02 (Variables|LEAVEMEALONE|GetYaw))) _lerp)))
        (:Finished
          (Variables|LEAVEMEALONE|SetcanMove true)
          (Utilities|FlowControl|Delay 0.2)
          (Variables|Default|SetcanBeDamaged true))))))

(event EventTick
  (params (DeltaSeconds :type Float%20%28single-precision%29))
  ;[0 0 1] Player Movement
  (if (Variables|LEAVEMEALONE|GetPCMovement)
    (Variables|LEAVEMEALONE|SetDeltaSeconds DeltaSeconds)
    (if (Variables|LEAVEMEALONE|GetcanMove)
      (bind _returndirection (CallFunction|PlayerMovement (Input|AxisValues|GetMoveRight) (Variables|LEAVEMEALONE|GetHorizontalSpeed)))
      (bind _returndirection_2 (CallFunction|PlayerMovement (Input|AxisValues|GetMoveUp) (Variables|LEAVEMEALONE|GetVerticalSpeed)))
      (Variables|LEAVEMEALONE|SetVerticalSpeed _returndirection_2)
      (Variables|LEAVEMEALONE|SetHorizontalSpeed _returndirection)
      (Transformation|SetActorLocation (+ (Transformation|GetActorLocation) (Math|Vector|RotateVector (Math|Vector|MakeVector 0.0 (Variables|LEAVEMEALONE|GetHorizontalSpeed) (Variables|LEAVEMEALONE|GetVerticalSpeed)) (Math|Rotator|MakeRotator 0.0 0.0 (Variables|LEAVEMEALONE|GetYaw)))) true false))))

(event Game|Damage|EventAnyDamage
  (params (Damage :type Float%20%28single-precision%29) (DamageType :type Damage%20Type%20Object%20Reference) (InstigatedBy :type Controller%20Object%20Reference) (DamageCauser :type Actor%20Object%20Reference))
  ;[1 0 0] Take Damage
  (if (Variables|Default|GetcanBeDamaged)
    (Variables|LEAVEMEALONE|SetPlayerHealth (Math|Float|Clamp(Float) (- (Variables|LEAVEMEALONE|GetPlayerHealth) Damage) 0.0 (Variables|AdjustableVariables|GetMaxHealth)))
    (if (<= (Variables|LEAVEMEALONE|GetPlayerHealth) 0.0)
      (Utilities|IsValid (stale Custom|UsePowerup _returnvalue_2)
        (:Is%20Valid
          (Actor|DestroyActor (stale Custom|UsePowerup _returnvalue_2))
          (Effects|SpawnEmitteratLocation "/Game/Assets/Particles/Explosion.Explosion" (Transformation|GetActorLocation))
          (Utilities|FlowControl|Delay 0.2)
          (Actor|DestroyActor))
        (:Is%20Not%20Valid
          (Effects|SpawnEmitteratLocation "/Game/Trevino_Content/Trevino_Particle/Trevino_Explosion.Trevino_Explosion" (Transformation|GetActorLocation))
          (Utilities|FlowControl|Delay 0.2)
          (Actor|DestroyActor))))))

(event Input|ActionEvents|InputActionUsePowerup
  (params (Key :type Key%20Structure :default "AnyKey"))
  ;[0 1 0] Powerup Event
  (:Pressed
    ;[0 1 0] Laser Powerup
    (if (== (Variables|LEAVEMEALONE|GetPowerupVar) 1)
      (bind _returnvalue (Game|SpawnActorfromClass "/Game/Blueprints/Projectiles/Player_Laser.Player_Laser_C" (Transformation|GetWorldTransform (Variables|Default|GetLaserSpawn)) "Undefined" 0 (Math|Color|MakeColor 0.0 0.0 0.0) self))
      (Variables|/Script/Engine.RotatingMovementComponent|SetRotationRate (Variables|/Game/Blueprints/Projectiles/Player_Laser.Player_Laser_C|GetRotatingMovement _returnvalue) "0, 0,360.000000")
      (Variables|LEAVEMEALONE|SetPowerupVar 0)
      (else
        ;[0 1 0] Ship Powerup
        (if (== (Variables|LEAVEMEALONE|GetPowerupVar) 2)
          (bind _returnvalue_2 (Game|SpawnActorfromClass "/Game/Blueprints/Powerups/Powerup_Pawn.Powerup_Pawn_C" (Math|Transform|MakeTransform (.Location (Math|Transform|BreakTransform (Transformation|GetWorldTransform (Variables|Default|GetPowerupShipSpawn)))) "0, 0, 0" "1.000000,1.000000,1.000000") "Undefined" 0 0))
          (Variables|LEAVEMEALONE|SetPowerupVar 0))))))

(event Input|ActionEvents|InputActionFire
  (params (Key :type Key%20Structure :default "AnyKey"))
  ;[1 0 0] Fire Timer
  (:Pressed
    (bind _returnvalue (Utilities|Time|SetTimerbyFunctionName 0 "FireReset" (Variables|AdjustableVariables|GetFireRate) true))
    (Variables|LEAVEMEALONE|SetTimeHandler _returnvalue)
    (CallFunction|PrimaryFire (Variables|Default|GetTopProjectileSpawn))
    (CallFunction|PrimaryFire (Variables|Default|GetBottomProjectileSpawn)))
  (:Released
    (Utilities|Time|ClearandInvalidateTimerbyHandle (Variables|LEAVEMEALONE|GetTimeHandler))))

(event Input|ActionEvents|InputActionSecondaryFire
  (params (Key :type Key%20Structure :default "AnyKey"))
  ;[1 0 0] FireLaser
  (:Pressed
    (if (Variables|LEAVEMEALONE|GetLaserReady)
      (Variables|LEAVEMEALONE|SetLaserReady false)
      (Game|SpawnActorfromClass "/Game/Blueprints/Projectiles/Player_Laser.Player_Laser_C" (Transformation|GetWorldTransform (Variables|Default|GetLaserSpawn)) "Undefined" 0 (Math|Color|MakeColor 0.2 0.2 1.0 1.0) self)
      (Timeline|Timeline_0 PlayFromStart
        (:Finished
          (Utilities|IsValid self
            (:Is%20Valid
              (Variables|LEAVEMEALONE|SetLaserReady true))
            (:Is%20Not%20Valid
              (CallFunction|Respawn))))))))

(fn ConstructionScript
  (Variables|LEAVEMEALONE|SetPlayerHealth (Variables|AdjustableVariables|GetMaxHealth)))

(fn PlayerMovement
  (params (Direction :type Float%20%28single-precision%29) (Speed :type Float%20%28single-precision%29))
  ;[0 0 1] Player Movement Function
  (bind _output_get (Variables|LEAVEMEALONE|SetCurrentSpeed (Math|Interpolation|FInterpTo Speed (* (* Direction (Variables|AdjustableVariables|GetMovementSpeed)) (Variables|LEAVEMEALONE|GetDeltaSeconds)) (Variables|LEAVEMEALONE|GetDeltaSeconds) 4.0)))
  (return _output_get))

(fn PrimaryFire
  (params (Location :type Scene%20Component%20Object%20Reference))
  ;[1 0 0] Primary Fire Function
  (Game|SpawnActorfromClass "/Game/Blueprints/Projectiles/Player_Projectile.Player_Projectile_C" (Transformation|GetWorldTransform Location) "Undefined" 0 (Math|Color|MakeColor 0.6 0.3 0.6 1.0) (Math|Vector|MakeVector 7e+02 0.0 0.0) self))